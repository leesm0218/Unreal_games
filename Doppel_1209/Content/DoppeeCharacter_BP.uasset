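; Doppee character Blueprint that can take a random body color and walk to a target location on demand.
; The construction script creates a dynamic material from the mesh's first slot, whose BodyColor SetColor randomizes.
; Move runs AIMoveTo toward TargetLocation; an Aborted failure applies a teleporting local offset derived from the target, then retries.
; That retry uses NewVar0 as its pawn, whose assignment never executes.
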(event `self.setColor`
  (`MaterialInstanceDynamic.SetVectorParameterValue` (`self.MyColor`) "BodyColor" (make `LinearColor` (`KismetMathLibrary.RandomFloat`) (`KismetMathLibrary.RandomFloat`) (`KismetMathLibrary.RandomFloat`) 1.0)))

(event `self.Move`
  (bind _targetlocation (`self.targetLocation`))
  (bind _returnvalue (`self.K2_GetActorLocation` self))
  (bind _returnvalue_2 (`AIBlueprintHelperLibrary.GetAIController` self))
  (bind _movementresult (`|AIMoveTo` (`Controller.K2_GetPawn` _returnvalue_2) _targetlocation)
    (:`OnFail`
      (switch `EPathFollowingResult` _movementresult
        (:`Aborted`
          (`self.K2_AddActorLocalOffset` (+ (* (- _targetlocation _returnvalue) (1.0 1.0 0.0)) (* _returnvalue (0.0 0.0 1.0))) false true)
          (`|AIMoveTo` (`self.NewVar_0`) (`self.targetLocation`)))))))

(fn `UserConstructionScript`
  (bind _mesh (`self.Mesh`))
  (bind _returnvalue (`PrimitiveComponent.CreateDynamicMaterialInstance` _mesh 0 (`KismetArrayLibrary.Array_Get` (`MeshComponent.GetMaterials` _mesh))))
  (set `self.MyColor` _returnvalue))