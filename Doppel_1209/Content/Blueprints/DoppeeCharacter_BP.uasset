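; DoppeeCharacter_BP is a character that hops to a target location and can take a random body color.
; The construction script creates a dynamic material instance on the mesh, whose BodyColor parameter SetColor randomizes.
; Move faces TargetLocation, launches the character toward it with a slight upward boost, then snaps it exactly there after a short delay.
; Turn, BeginPlay, overlap and Tick are empty, and Move's AI controller lookup goes unused.
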(event `self.setColor`
  (`MaterialInstanceDynamic.SetVectorParameterValue` (`self.MyColor`) "BodyColor" (make `LinearColor` (`KismetMathLibrary.RandomFloat`) (`KismetMathLibrary.RandomFloat`) (`KismetMathLibrary.RandomFloat`) 1.0)))

(event `self.Move`
  (bind _returnvalue (- (`self.targetLocation`) (`self.K2_GetActorLocation`)))
  (`AIBlueprintHelperLibrary.GetAIController` self)
  (`self.K2_SetActorRotation` (`KismetMathLibrary.Conv_VectorToRotator` _returnvalue))
  (`self.LaunchCharacter` (+ (* _returnvalue 5.0) (0.0 0.0 50.0)))
  (`KismetSystemLibrary.Delay` 0.75)
  (`self.K2_SetActorLocation` (`self.targetLocation`)))

(event `self.Turn`)

(fn `UserConstructionScript`
  (bind _mesh (`self.Mesh`))
  (bind _returnvalue (`PrimitiveComponent.CreateDynamicMaterialInstance` _mesh 0 (`KismetArrayLibrary.Array_Get` (`MeshComponent.GetMaterials` _mesh))))
  (set `self.MyColor` _returnvalue))